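; AI controller for the stag and doe animals that runs their behavior tree and blackboard, flagging fruit eating when the pawn is a stag.
; AI perception writes sensed actors of a different class into the character blackboard key, records their distance, and clears the key on any lost stimulus.
; SetupAppleNotification lets an apple reference be written to the food blackboard key.
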(event `self.ReceiveBeginPlay`
  (`self.RunBehaviorTree` "/Game/Animals/DeerStagAndDoe/Blueprints/BT_AnimalBehavior.BT_AnimalBehavior")
  (bind _blackboardcomponent (`self.UseBlackboard` "/Game/Animals/DeerStagAndDoe/Blueprints/Animal_Blackboard.Animal_Blackboard"))
  (set `self.BlackboardComponent` _blackboardcomponent)
  (cast `/Game/Animals/DeerStagAndDoe/Blueprints/BP_Stag` (`self.K2_GetPawn`))
  (set `self.EatsFruit?` true))

(event `self.AIPerception.OnTargetPerceptionUpdated`
  (params (Actor :type "Actor Object Reference") (Stimulus :type "AIStimulus Structure"))
  (if Stimulus_bSuccessfullySensed
    (if (not (== (`GameplayStatics.GetObjectClass` (`self.K2_GetPawn`)) (`GameplayStatics.GetObjectClass` Actor)))
      (set `self.DistanceFromCharacter` (`KismetMathLibrary.Vector_Distance` (`self.K2_GetActorLocation` (`self.K2_GetPawn`)) Stimulus_StimulusLocation))
      (`BlackboardComponent.SetValueAsObject` (`self.BlackboardComponent`) (`self.BlackBoardCharacterKey`) Actor))
    (else
      (`BlackboardComponent.ClearValue` (`self.BlackboardComponent`) (`self.BlackBoardCharacterKey`)))))

(fn `Setup Apple Notification`
  (params (AppleReference :type "/Game/Props/Blueprints/BP_Apple Object Reference"))
  (`BlackboardComponent.SetValueAsObject` (`self.BlackboardComponent`) (`self.BlackBoardFoodKey`) AppleReference))

(fn `UserConstructionScript`)
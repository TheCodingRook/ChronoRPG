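; Fire interaction logic owned by a brazier that passes flame between it and a torch attached to the instigator.
; LightFire searches the instigator's attached actors for a BP_Torch and, when only one of torch or brazier is lit, lights the other.
; Either outcome removes the related prompt widget and pops this interaction command from ChronoRPGGameInstance.
; Lighting the brazier also calls its OnWasInteractedWith and flags its widget as unnecessary.
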(event `self.LightFire`
  (params (Instigator :type "ChronoRPGCharacter Object Reference"))
  (bind _brazier (`self.Brazier`))
  (bind _asbp_brazier (cast `/Game/Props/Blueprints/BP_Brazier` (`self.GetOwner`)))
  (set `self.Brazier` _asbp_brazier)
  (for _array_element (`Actor.GetAttachedActors` Instigator true)
    (bind _asbp_torch (cast `/Game/Props/Blueprints/BP_Torch` _array_element))
    (bind _output_get (set `self.Torch` _asbp_torch))
    (if (xor (`/Game/Props/Blueprints/BP_Torch.IsLit?` _output_get) (`/Game/Props/Blueprints/BP_Brazier.IsLit?` (`self.Brazier`)))
      (`|ExecutionSequence`
        (:`then_0`
          (if (not (`/Game/Props/Blueprints/BP_Brazier.IsLit?` (`self.Brazier`)))
            (`/Game/Props/Blueprints/BP_Brazier.ToggleFire` _brazier)
            (`InteractablePropBase.OnWasInteractedWith` _brazier)
            (set `/Game/Props/Blueprints/BP_InteractableProp.IsWidgetNecessary?` false _brazier)
            (`Widget.RemoveFromParent` (`/Game/Props/Blueprints/BP_InteractableProp.InteractionWidget` _brazier))
            (bind _aschrono_rpggame_instance (cast `ChronoRPGGameInstance` (`GameplayStatics.GetGameInstance`) :!label _label))
            (`ChronoRPGGameInstance.PopInteractionCommand` _aschrono_rpggame_instance self)))
        (:`then_1`
          (if (not (`/Game/Props/Blueprints/BP_Torch.IsLit?` (`self.Torch`)))
            (`/Game/Props/Blueprints/BP_Torch.ToggleFire` (`self.Torch`))
            (`Widget.RemoveFromParent` (`/Game/Props/Blueprints/BP_Brazier.TorchWidget` (`self.Brazier`)))
            (goto _label)))))))
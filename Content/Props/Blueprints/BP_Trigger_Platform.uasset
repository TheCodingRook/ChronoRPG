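; BP_Trigger_Platform is a pressure plate prop that acts as a trigger for puzzles.
; Its collision volume tracks overlapping actors that implement the ActivateTriggerPlatform interface.
; The first actor on fires the PuzzleElement triggered call, plays a grinding sound and runs a timeline that lerps the platform slightly down.
; When the last actor leaves, it fires the untriggered call, replays the sound and reverses the timeline.
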(event `self.ReceiveBeginPlay`
  (set `self.StartingLocation` (`self.K2_GetActorLocation`)))

(event `self.CollisionVolume.OnComponentBeginOverlap`
  (params (OverlappedComponent :type "PrimitiveComponent Object Reference") (OtherActor :type "Actor Object Reference") (OtherComp :type "PrimitiveComponent Object Reference") (OtherBodyIndex :type Integer) (bFromSweep :type Boolean) (SweepResult :type "HitResult Structure (by ref)"))
  (bind (_startinglocation_x _startinglocation_y) (`KismetMathLibrary.BreakVector` (`self.StartingLocation`)))
  (bind (_startinglocation_x_2 _startinglocation_y_2 _startinglocation_z) (`KismetMathLibrary.BreakVector` (`self.StartingLocation`)))
  (if (`KismetSystemLibrary.DoesImplementInterface` OtherActor "/Script/ChronoRPG.ActivateTriggerPlatform")
    ;[0 0.7891 1] Let's keep track of how many actors are pressing down
    (`KismetArrayLibrary.Array_AddUnique` (`self.OverlappingActors`) OtherActor)
    (if (== (`KismetArrayLibrary.Array_Length` (`self.OverlappingActors`)) 1)
      (`PuzzleElementComponent.OnPuzzleElementTriggered` (`self.PuzzleElement`))
      (`GameplayStatics.PlaySoundAtLocation` "/Game/Audio/GrindingStone.GrindingStone" (`self.K2_GetActorLocation` self) (struct) 1.0 1.0 0.0 null null null)
      (bind (_direction _alpha) (`Timeline|Press Down Speed` :!label _label)
        (:`Update`
          (`self.K2_SetActorLocation` (`KismetMathLibrary.MakeVector` _startinglocation_x _startinglocation_y (`KismetMathLibrary.Lerp` _startinglocation_z (+ _startinglocation_z -5.0) _alpha))))))))

(event `self.CollisionVolume.OnComponentEndOverlap`
  (params (OverlappedComponent :type "PrimitiveComponent Object Reference") (OtherActor :type "Actor Object Reference") (OtherComp :type "PrimitiveComponent Object Reference") (OtherBodyIndex :type Integer))
  (if (`KismetSystemLibrary.DoesImplementInterface` OtherActor "/Script/ChronoRPG.ActivateTriggerPlatform")
    (`KismetArrayLibrary.Array_RemoveItem` (`self.OverlappingActors`) OtherActor)
    (if (== (`KismetArrayLibrary.Array_Length` (`self.OverlappingActors`)) 0)
      (`PuzzleElementComponent.OnPuzzleElementUnTriggered` (`self.PuzzleElement`))
      (`GameplayStatics.PlaySoundAtLocation` "/Game/Audio/GrindingStone.GrindingStone" (`self.K2_GetActorLocation` self) (struct) 1.0 1.0 0.0 null null null)
      (goto _label :!via `Reverse`))))

(fn `UserConstructionScript`)
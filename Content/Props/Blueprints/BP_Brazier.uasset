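; BP_Brazier is a brazier prop with toggleable fire that prompts the player to light a torch from it.
; When an unlit BP_Torch enters TorchTrigger while the brazier is lit, a once-created WBP_InteractionPrompt is shown, then removed on exit.
; ToggleFire flips fire and light visibility along with the lit state.
; QueryPropCombo reports whether the character carries a lit torch, checking only the first attached actor.
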(event `self.TorchTrigger.OnComponentBeginOverlap`
  (params (OverlappedComponent :type "PrimitiveComponent Object Reference") (OtherActor :type "Actor Object Reference") (OtherComp :type "PrimitiveComponent Object Reference") (OtherBodyIndex :type Integer) (bFromSweep :type Boolean) (SweepResult :type "HitResult Structure (by ref)"))
  (bind _torchwidget (`self.TorchWidget`))
  (bind _asbp_torch (cast `/Game/Props/Blueprints/BP_Torch` OtherActor))
  (if (`/Game/Props/Blueprints/BP_Torch.IsLit?` _asbp_torch)
    _
    (elif (`self.IsLit?`)
      (`|ExecutionSequence`
        (:`then_0`
          (`/Engine/EditorBlueprintResources/StandardMacros.DoOnce` false
            (:`Completed`
              (bind _returnvalue (`|CreateWidget` "/Game/UI/Blueprints/WBP_InteractionPrompt.WBP_InteractionPrompt_C" (`GameplayStatics.GetPlayerController` 0)))
              (bind _output_get (set `self.TorchWidget` _returnvalue))
              (set `/Game/UI/Blueprints/WBP_InteractionPrompt.InteractionText` "LIGHT TORCH" _output_get)
              (set `/Game/UI/Blueprints/WBP_InteractionPrompt.InteractableActor` self _torchwidget)
              (`UserWidget.AddToViewport` _torchwidget 0))))
        (:`then_1`
          (if (not (`Widget.IsInViewport` (`self.TorchWidget`)))
            (`UserWidget.AddToViewport` (`self.TorchWidget`) 0)))))))

(event `self.TorchTrigger.OnComponentEndOverlap`
  (params (OverlappedComponent :type "PrimitiveComponent Object Reference") (OtherActor :type "Actor Object Reference") (OtherComp :type "PrimitiveComponent Object Reference") (OtherBodyIndex :type Integer))
  (bind _torchwidget (`self.TorchWidget`))
  (cast `/Game/Props/Blueprints/BP_Torch` OtherActor)
  (`/Engine/EditorBlueprintResources/StandardMacros.IsValid` _torchwidget
    (:`Is Valid`
      (`Widget.RemoveFromParent` _torchwidget))))

(fn `QueryPropCombo`
  (params (InBP_ChronoRPGCharacter :type "/Game/Player/Blueprints/BP_ChronoRPGCharacter Object Reference"))
  (returns (ActionAvailability :type Boolean))
  (for _array_element (`self.GetAttachedActors` InBP_ChronoRPGCharacter true)
    (bind _asbp_torch (cast `/Game/Props/Blueprints/BP_Torch` _array_element)
      (:`then`
        (return (`/Game/Props/Blueprints/BP_Torch.IsLit?` _asbp_torch)))
      (:`CastFailed`
        (return false))))
  (return false))

(fn `ToggleFire`
  (bind _returnvalue (not (`self.IsLit?`)))
  (`SceneComponent.SetVisibility` (`self.Fire`) (not (`self.IsLit?`)) false)
  (`SceneComponent.SetVisibility` (`self.PointLight`) (not (`self.IsLit?`)) false)
  (set `self.IsLit?` _returnvalue)
  (set `self.IsWidgetNecessary?` _returnvalue))

(fn `UserConstructionScript`
  (`parent.UserConstructionScript`))
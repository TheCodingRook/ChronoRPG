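; Time portal prop that teleports the player character to TeleportLocation and shows a camera-driven portal view.
; Each Tick, PortalSceneCapture copies the player camera's rotation with a yaw offset derived from trigger and destination.
; PortalTrigger broadcasts OnPortalTraversal on any overlap, but only teleports on character mesh overlap while active, aligning control yaw to the destination.
; AllowThroughToggle deactivates the portal while the character overlaps it, re-enabling after a short delay.
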(event `self.ReceiveTick`
  (params (DeltaSeconds :type "Float (single-precision)"))
  (bind (_returnvalue_roll _returnvalue_pitch _returnvalue_yaw) (`KismetMathLibrary.BreakRotator` (`SceneComponent.K2_GetComponentRotation` (`self.PortalTrigger`))))
  (bind (_returnvalue_roll_2 _returnvalue_pitch_2 _returnvalue_yaw_2) (`KismetMathLibrary.BreakRotator` (`SceneComponent.K2_GetComponentRotation` (`self.TeleportLocation`))))
  (bind (_returnvalue_roll_3 _returnvalue_pitch_3 _returnvalue_yaw_3) (`KismetMathLibrary.BreakRotator` (`SceneComponent.K2_GetComponentRotation` (`PlayerCameraManager.TransformComponent` (`PlayerController.PlayerCameraManager` (`GameplayStatics.GetPlayerController` 0))))))
  (`SceneComponent.K2_SetWorldRotation` (`self.PortalSceneCapture`) (`KismetMathLibrary.MakeRotator` _returnvalue_roll_3 _returnvalue_pitch_3 (+ _returnvalue_yaw_3 (`KismetMathLibrary.Abs` (- (- _returnvalue_yaw_2 _returnvalue_yaw) 135.0)))) false false))

(event `self.AllowThroughToggle.OnComponentBeginOverlap`
  (params (OverlappedComponent :type "PrimitiveComponent Object Reference") (OtherActor :type "Actor Object Reference") (OtherComp :type "PrimitiveComponent Object Reference") (OtherBodyIndex :type Integer) (bFromSweep :type Boolean) (SweepResult :type "HitResult Structure (by ref)"))
  (cast `ChronoRPGCharacter` OtherActor)
  (set `self.bIsActive` false))

(event `self.AllowThroughToggle.OnComponentEndOverlap`
  (params (OverlappedComponent :type "PrimitiveComponent Object Reference") (OtherActor :type "Actor Object Reference") (OtherComp :type "PrimitiveComponent Object Reference") (OtherBodyIndex :type Integer))
  (cast `ChronoRPGCharacter` OtherActor)
  (`KismetSystemLibrary.Delay` 0.5)
  (set `self.bIsActive` true))

(event `self.PortalTrigger.OnComponentBeginOverlap`
  (params (OverlappedComponent :type "PrimitiveComponent Object Reference") (OtherActor :type "Actor Object Reference") (OtherComp :type "PrimitiveComponent Object Reference") (OtherBodyIndex :type Integer) (bFromSweep :type Boolean) (SweepResult :type "HitResult Structure (by ref)"))
  (bind _teleportlocation (`self.TeleportLocation`))
  (bind _returnvalue (`SceneComponent.K2_GetComponentRotation` _teleportlocation))
  (`self.OnPortalTraversal`) ; Send a notifier to all listeners
  (bind _asbp_chrono_rpgcharacter (cast `/Game/Player/Blueprints/BP_ChronoRPGCharacter` OtherActor))
  (if (and (`self.bIsActive`) (== OtherComp (`Character.Mesh` _asbp_chrono_rpgcharacter)))
    (`self.K2_SetActorLocationAndRotation` _asbp_chrono_rpgcharacter (`SceneComponent.K2_GetComponentLocation` _teleportlocation) _returnvalue false false)
    (bind _returnvalue_2 (`ChronoRPGCharacter.GetMyChronoRPGPlayerController` _asbp_chrono_rpgcharacter))
    (`Controller.SetControlRotation` _returnvalue_2 (`KismetMathLibrary.MakeRotator` (.roll (`Controller.GetControlRotation` _returnvalue_2)) (.pitch (`Controller.GetControlRotation` _returnvalue_2)) (.yaw _returnvalue)))))

(fn `UserConstructionScript`)
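; BP_Door is a puzzle-driven door that lowers when a linked puzzle element is triggered and rises back when it is untriggered.
; On BeginPlay it stores the door's world location and binds to the PuzzleElementComponent events of every actor in its Puzzle's list.
; The DoorSpeed timeline lerps the door's Z downward, playing to open and reversing to close.
; Each element drives the timeline independently, with no check that all are triggered.
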(event `self.ReceiveBeginPlay`
  (set `self.StartingLocation` (`SceneComponent.K2_GetComponentLocation` (`self.Door`)))
  (for _array_element (`PuzzleComponent.GetActorsList` (`self.Puzzle`))
    (bind _returnvalue (`self.GetComponentByClass` _array_element "/Script/ChronoRPG.PuzzleElementComponent"))
    (add `PuzzleElementComponent.OnPuzzleElementTriggered` _returnvalue (delegate `Move Door`))
    (add `PuzzleElementComponent.OnPuzzleElementUnTriggered` _returnvalue (delegate `Move Door Back`))))

(event `Move Door`
  (bind (_startinglocation_x _startinglocation_y) (`KismetMathLibrary.BreakVector` (`self.StartingLocation`)))
  (bind (_startinglocation_x_2 _startinglocation_y_2 _startinglocation_z) (`KismetMathLibrary.BreakVector` (`self.StartingLocation`)))
  (bind (_direction _alpha) (`Timeline|Door speed` :!label _label)
    (:`Update`
      (`SceneComponent.K2_SetWorldLocation` (`self.Door`) (`KismetMathLibrary.MakeVector` _startinglocation_x _startinglocation_y (`KismetMathLibrary.Lerp` _startinglocation_z (+ _startinglocation_z -200.0) _alpha)) false false))))

(event `Move Door Back`
  (goto _label :!via `Reverse`))

(fn `UserConstructionScript`)
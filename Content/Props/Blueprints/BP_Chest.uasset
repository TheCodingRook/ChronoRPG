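; BP_Chest is a lockable chest prop that pairs with a BP_Key carried by the RPG character.
; QueryPropCombo searches the character's attached actors for a key, and InsertKey snaps a given key onto the lock's KeySocket.
; OpenLid offsets the lid's rotation and location instantly, removes the interaction widget and flags the chest as unlocked.
; The event graph is empty, so nothing in this Blueprint calls these functions.
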(fn `InsertKey`
  (params (KeyToUse :type "/Game/Props/Blueprints/BP_Key Object Reference"))
  (`self.K2_AttachToComponent` KeyToUse (`self.Lock`) "KeySocket" "SnapToTarget" "SnapToTarget" "SnapToTarget" true))

(fn `OpenLid`
  (`SceneComponent.K2_AddRelativeRotation` (`self.Lid`) (struct :`Pitch` 50.0) false false)
  (`SceneComponent.K2_AddRelativeLocation` (`self.Lid`) (-10.0 0.0 27.0) false false)
  (`Widget.RemoveFromParent` (`self.InteractionWidget`))
  (set `self.IsWidgetNecessary?` false)
  (set `self.IsAlreadyUnlocked?` true))

(fn `QueryPropCombo`
  (params (InBP_ChronoRPGCharacter :type "/Game/Player/Blueprints/BP_ChronoRPGCharacter Object Reference"))
  (returns (ActionAvailability :type Boolean))
  (locals (`FoundKey?` :type Boolean))
  (for _array_element (`self.GetAttachedActors` InBP_ChronoRPGCharacter true)
    (cast `/Game/Props/Blueprints/BP_Key` _array_element)
    (set `local.FoundKey?` true))
  (return (`local.FoundKey?`)))

(fn `UserConstructionScript`
  (`parent.UserConstructionScript`))
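; Interaction component that lets a character unlock its owning chest with a carried key.
; UnlockProp checks that the BP_Chest is still locked, searches the instigator's attached actors for a BP_Key and opens the lid.
; DropKey then releases the key through the grabbing ability, pops its interaction command from the game instance, removes its widget and inserts it into the chest.
; The logic is hard-cast to BP_Chest, flagged in the graph as too specific.
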(event `self.UnlockProp`
  (params (Instigator :type "ChronoRPGCharacter Object Reference"))
  (set `self.InstigatorRef` Instigator)
  (bind _asbp_chest (cast `/Game/Props/Blueprints/BP_Chest` (`self.GetOwner`))) ; THIS IS TOO SPECIFIC TO BP_CHEST!!
  (bind _output_get (set `self.Chest` _asbp_chest))
  (if (not (`/Game/Props/Blueprints/BP_Chest.IsAlreadyUnlocked?` _output_get))
    (for _array_element (`Actor.GetAttachedActors` Instigator true)
      (bind _asbp_key (cast `/Game/Props/Blueprints/BP_Key` _array_element))
      (set `self.Key` _asbp_key)
      (`/Game/Props/Blueprints/BP_Chest.OpenLid` (`self.Chest`))
      (`self.DropKey` (`self.InstigatorRef`)))))

(fn `DropKey`
  (params (InChronoRPGCharacter :type "ChronoRPGCharacter Object Reference"))
  (bind _key (`self.Key`))
  (bind _asbp_chrono_rpgcharacter (cast `/Game/Player/Blueprints/BP_ChronoRPGCharacter` InChronoRPGCharacter))
  (`GrabbingAbility.DropProp` (`/Game/Player/Blueprints/BP_ChronoRPGCharacter.GrabbingAbility` _asbp_chrono_rpgcharacter))
  (bind _aschrono_rpggame_instance (cast `ChronoRPGGameInstance` (`GameplayStatics.GetGameInstance`)))
  (`ChronoRPGGameInstance.PopInteractionCommand` _aschrono_rpggame_instance (`InteractablePropBase.GetInteractionCommand` (`self.Key`)))
  (`Widget.RemoveFromParent` (`/Game/Props/Blueprints/BP_InteractableProp.InteractionWidget` _key))
  (set `/Game/Props/Blueprints/BP_InteractableProp.IsWidgetNecessary?` false _key)
  (`/Game/Props/Blueprints/BP_Chest.InsertKey` (`self.Chest`) (`self.Key`)))
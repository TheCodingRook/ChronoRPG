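; Apple spawner actor that drops apples at random points inside its box volume on a looping timer, its interval randomized once at BeginPlay.
; It reuses apples from the GameInstance's shared pool, spawning new ones up to MaxApples only when that pool is empty.
; Newly spawned apples bind their fall event to notify the BP_Stag's AI controller.
; An earlier local pool with gate control remains but is never started.
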(event `NofityAnimal`
  (bind _returnvalue (`GameplayStatics.GetActorOfClass` "/Game/Animals/DeerStagAndDoe/Blueprints/BP_Stag.BP_Stag_C"))
  (bind _asbp_animal_aicontroller (cast `/Game/Animals/DeerStagAndDoe/Blueprints/BP_AnimalAIController` (`Pawn.GetController` _returnvalue)))
  (`/Game/Animals/DeerStagAndDoe/Blueprints/BP_AnimalAIController.Setup Apple Notification` _asbp_animal_aicontroller (stale `SpawnApple` _returnvalue)))

(event `self.ReceiveBeginPlay`
  (`KismetSystemLibrary.K2_SetTimerDelegate` (delegate `SpawnApple`) (* (`KismetMathLibrary.RandomFloat`) (`self.MaxSpawnDelay`)) true))

(event `SpawnApple`
  (bind _aschrono_rpggame_instance (cast `ChronoRPGGameInstance` (`GameplayStatics.GetGameInstance`)))
  (bind _applepool (`ChronoRPGGameInstance.ApplePool` _aschrono_rpggame_instance))
  (set `self.AppleActorPool` _applepool)
  (if (== (`ActorPool.PoolSize` _applepool) 0)
    (if (< (`self.AppleCounter`) (`self.MaxApples`))
      (bind _returnvalue (`|SpawnActorFromClass` "/Game/Props/Blueprints/BP_Apple.BP_Apple_C" (`KismetMathLibrary.MakeTransform` (`KismetMathLibrary.TransformLocation` (`SceneComponent.K2_GetComponentToWorld` (`self.Box`)) (`KismetMathLibrary.RandomPointInBoundingBox` (0.0 0.0 0.0) (`BoxComponent.BoxExtent` (`self.Box`)))) (`KismetMathLibrary.RandomRotator` true)) "AlwaysSpawn" "OverrideRootScale" self null))
      (add `/Game/Props/Blueprints/BP_Apple.OnAppleFell` _returnvalue (delegate `NofityAnimal`))
      (`/Engine/EditorBlueprintResources/StandardMacros.IncrementInt` (`self.AppleCounter`)
        (:`  `
          (`/Game/Props/Blueprints/BP_Apple.LiveYourLife` _returnvalue (`self.AppleLifeSpan`)))))
    (else
      (bind _returnvalue_2 (`ActorPool.CheckOut` (`self.AppleActorPool`)))
      (bind _asbp_apple (cast `/Game/Props/Blueprints/BP_Apple` _returnvalue_2 :!pure true))
      (`self.SetActorHiddenInGame` _asbp_apple false)
      (`PrimitiveComponent.SetSimulatePhysics` (`InteractablePropBase.GetMesh` _asbp_apple) true)
      (`self.K2_SetActorTransform` _asbp_apple (`KismetMathLibrary.MakeTransform` (`KismetMathLibrary.TransformLocation` (`SceneComponent.K2_GetComponentToWorld` (`self.Box`)) (`KismetMathLibrary.RandomPointInBoundingBox` (0.0 0.0 0.0) (`BoxComponent.BoxExtent` (`self.Box`)))) (`KismetMathLibrary.RandomRotator` true)) false true)
      (`/Game/Props/Blueprints/BP_Apple.LiveYourLife` _asbp_apple (`self.AppleLifeSpan`)))))

(event `EnterGate`
  ;[0 0.1562 1] ORIGINAL METHOD
  (`/Engine/EditorBlueprintResources/StandardMacros.Gate` false :!label _label
    (:`Exit`
      (bind _spawnedapple (`self.CheckOutApple` (`KismetMathLibrary.MakeTransform` (`KismetMathLibrary.TransformLocation` (`SceneComponent.K2_GetComponentToWorld` (`self.Box`)) (`KismetMathLibrary.RandomPointInBoundingBox` (0.0 0.0 0.0) (`BoxComponent.BoxExtent` (`self.Box`)))) (`KismetMathLibrary.RandomRotator` true))))
      (`self.AppleDebug` _spawnedapple "spawned")
      (`/Game/Props/Blueprints/BP_Apple.LiveYourLife` _spawnedapple (`self.AppleLifeSpan`)))))

(event `OpenGate`
  ;[0 0.1562 1] ORIGINAL METHOD
  (goto _label :!via `Open`))

(event `CloseGate`
  ;[0 0.1562 1] ORIGINAL METHOD
  (goto _label :!via `Close`))

(fn `AppleDebug`
  (params (Apple :type "/Game/Props/Blueprints/BP_Apple Object Reference") (Verb :type String))
  (`KismetSystemLibrary.PrintString` (`KismetStringLibrary.Concat_StrStr` (`KismetSystemLibrary.GetDisplayName` Apple) ":" Verb " at" "" (`KismetStringLibrary.Conv_DoubleToString` (`KismetSystemLibrary.GetGameTimeInSeconds`)))))

(fn `ApplePoolInitializer`
  (bind _returnvalue (`KismetArrayLibrary.Array_Length` (`self.ApplePool`)))
  ;[0 0.1562 1] Populate the Apple pool at BeginPlay
  (while (< _returnvalue (`self.MaxApples`))
    (bind _returnvalue_2 (`|SpawnActorFromClass` "/Game/Props/Blueprints/BP_Apple.BP_Apple_C" (`KismetMathLibrary.MakeTransform` (0.0 0.0 0.0)) "AlwaysSpawn" "OverrideRootScale" self null))
    (`KismetArrayLibrary.Array_AddUnique` (`self.ApplePool`) _returnvalue_2)
    (`KismetSystemLibrary.PrintString` (`KismetStringLibrary.Conv_IntToString` _returnvalue))))

(fn `CheckInApple`
  (params (AppleToCheckIn :type "/Game/Props/Blueprints/BP_Apple Object Reference"))
  ;[0 0.4609 1] Disable physics and hide actors
  (`PrimitiveComponent.SetSimulatePhysics` (`InteractablePropBase.GetMesh` AppleToCheckIn) false)
  (`self.K2_SetActorLocation` AppleToCheckIn (0.0 0.0 0.0) false true)
  (`self.SetActorHiddenInGame` AppleToCheckIn true)
  (`KismetArrayLibrary.Array_AddUnique` (`self.ApplePool`) AppleToCheckIn))

(fn `CheckOutApple`
  (params (InTransform :type "Transform Structure"))
  (returns (SpawnedApple :type "/Game/Props/Blueprints/BP_Apple Object Reference"))
  (locals (AppleToSpawn :type "/Game/Props/Blueprints/BP_Apple Object Reference") (AppleKeyToSpawn :type Integer))
  (set `local.AppleToSpawn` (`|GetArrayItem` (`self.ApplePool`)))
  ;[0 1 0.4141] Make apple visible, enable physics and put it back in the world
  (`self.SetActorHiddenInGame` (`local.AppleToSpawn`) false)
  (`PrimitiveComponent.SetSimulatePhysics` (`InteractablePropBase.GetMesh` (`local.AppleToSpawn`)) true)
  (`self.K2_SetActorTransform` (`local.AppleToSpawn`) InTransform false false)
  (`KismetArrayLibrary.Array_Remove` (`self.ApplePool`))
  ;[0 0.2031 1] Close the control Gate if we emptied the actor pool
  (if (== (`KismetArrayLibrary.Array_Length` (`self.ApplePool`)) 0)
    (`self.CloseGate`)
    (`KismetSystemLibrary.PrintString` "Gate Closed"))
  (return (`local.AppleToSpawn`)))

(fn `UserConstructionScript`)
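; BP_Torch is a torch prop that can be switched between lit and unlit.
; ToggleFire sets the visibility of the Fire and PointLight components to the inverse of IsLit, without propagating to children, then flips that flag.
; The event graph holds only disabled default events and the construction script only calls its parent, so nothing in this Blueprint calls the toggle itself.
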(fn `ToggleFire`
  (bind _returnvalue (not (`self.IsLit?`)))
  (`SceneComponent.SetVisibility` (`self.Fire`) (not (`self.IsLit?`)) false)
  (`SceneComponent.SetVisibility` (`self.PointLight`) _returnvalue false)
  (set `self.IsLit?` _returnvalue))

(fn `UserConstructionScript`
  (`parent.UserConstructionScript`))
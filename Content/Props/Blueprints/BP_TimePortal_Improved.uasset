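; BP_TimePortal_Improved is a portal actor that aims a scene capture to follow the player's view.
; Each Tick sets PortalSceneCapture's rotation from the player camera's roll and pitch, with yaw offset by PortalTrigger and TeleportLocation yaws and flipped 180 degrees.
; Tick also prints a debug yaw sum on screen.
; Capture location is never updated, the position-offset math is unconnected, and no overlap or teleport logic is implemented.
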(event `self.ReceiveTick`
  (params (DeltaSeconds :type "Float (single-precision)"))
  (bind (_returnvalue_roll _returnvalue_pitch _returnvalue_yaw) (`KismetMathLibrary.BreakRotator` (`SceneComponent.K2_GetComponentRotation` (`self.PortalTrigger`))))
  (bind (_returnvalue_roll_2 _returnvalue_pitch_2 _returnvalue_yaw_2) (`KismetMathLibrary.BreakRotator` (`SceneComponent.K2_GetComponentRotation` (`self.TeleportLocation`))))
  (bind (_returnvalue_roll_3 _returnvalue_pitch_3 _returnvalue_yaw_3) (`KismetMathLibrary.BreakRotator` (`SceneComponent.K2_GetComponentRotation` (`PlayerCameraManager.TransformComponent` (`PlayerController.PlayerCameraManager` (`GameplayStatics.GetPlayerController` 0))))))
  (bind _returnvalue (+ _returnvalue_yaw_3 _returnvalue_yaw))
  (`KismetSystemLibrary.PrintString` (`KismetStringLibrary.Conv_DoubleToString` _returnvalue) true true (struct :`G` 0.66 :`B` 1.0 :`A` 1.0) 0.001)
  (`SceneComponent.K2_SetWorldRotation` (`self.PortalSceneCapture`) (`KismetMathLibrary.MakeRotator` _returnvalue_roll_3 _returnvalue_pitch_3 (- (+ _returnvalue _returnvalue_yaw_2) 180.0)) false false))

(fn `UserConstructionScript`)